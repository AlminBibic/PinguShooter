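; Game mode that runs the match: a countdown timer against the number of Pingus still alive, deciding win or loss.
; Tick feeds a one-second Delay that decrements Minutes and Seconds, and reaching zero with Pingus left shows the lose screen.
; A parallel per-tick check shows the win screen when PingusAlive hits zero.
; Either outcome shows the cursor, disables player movement and sets IsGameOver.
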(event `self.ReceiveTick`
  (params (DeltaSeconds :type "Float (single-precision)"))
  (`|ExecutionSequence`
    (:`then_0`
      (`KismetSystemLibrary.Delay` 1.0)
      (set `self.Seconds` (- (`self.Seconds`) 1))
      (if (< (`self.Seconds`) 0)
        (set `self.Minutes` (- (`self.Minutes`) 1))
        (set `self.Seconds` 59))
      (if (== (`self.Seconds`) 0)
        (if (== (`self.Minutes`) 0)
          (bind _asbp_game_mode (cast `/Game/Blueprints/BP_GameMode` (`GameplayStatics.GetGameMode`)))
          (if (> (`/Game/Blueprints/BP_GameMode.PingusAlive` _asbp_game_mode) 0)
            (bind _returnvalue (`|CreateWidget` "/Game/Blueprints/WBP_LoseScreen.WBP_LoseScreen_C"))
            (`UserWidget.AddToViewport` _returnvalue 0)
            (set `PlayerController.bShowMouseCursor` true (`GameplayStatics.GetPlayerController` 0))
            (bind _asbp_player (cast `/Game/Blueprints/BP_Player` (`GameplayStatics.GetPlayerPawn` 0)))
            (`CharacterMovementComponent.DisableMovement` (`Character.CharacterMovement` _asbp_player))
            (set `self.IsGameOver` true)))))
    (:`then_1`
      (if (== (`/Game/Blueprints/BP_GameMode.PingusAlive` (stale `self.ReceiveBeginPlay` _asbp_game_mode)) 0)
        (bind _returnvalue_2 (`|CreateWidget` "/Game/Blueprints/WBP_WinScreen.WBP_WinScreen_C"))
        (`UserWidget.AddToViewport` _returnvalue_2 0)
        (set `PlayerController.bShowMouseCursor` true (`GameplayStatics.GetPlayerController` 0))
        (bind _asbp_player_2 (cast `/Game/Blueprints/BP_Player` (`GameplayStatics.GetPlayerPawn` 0)))
        (`CharacterMovementComponent.DisableMovement` (`Character.CharacterMovement` _asbp_player_2))
        (set `self.IsGameOver` true)))))

(event `self.ReceiveBeginPlay`
  (bind _asbp_game_mode (cast `/Game/Blueprints/BP_GameMode` (`GameplayStatics.GetGameMode`))))

(fn `UserConstructionScript`)