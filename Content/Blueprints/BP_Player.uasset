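; BP_Player is a player Blueprint that aims up or down and launches fish projectiles with Space.
; Up and Down keys pitch Arrow1 and adjust a Float variable that sets the vertical launch impulse.
; Space spawns a scaled-down BP_Projectile at ProjectileSpawnPoint and pushes its Fish component with a fixed negative-X impulse plus that vertical value, in world axes.
; An alternative AddImpulseAtLocation call is left unconnected.
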(event `Key|Up`
  (params (Key :type "Key Structure"))
  (bind _arrow1 (`self.Arrow1`))
  (bind (_returnvalue_roll _returnvalue_pitch) (`KismetMathLibrary.BreakRotator` (`SceneComponent.K2_GetComponentRotation` _arrow1)))
  (:`Pressed`
    (`SceneComponent.K2_SetRelativeRotation` _arrow1 (`KismetMathLibrary.MakeRotator` _returnvalue_roll (+ _returnvalue_pitch 2.0) 0.0) false false)
    (set `self.Float` (+ (`self.Float`) 50.0))))

(event `Key|Down`
  (params (Key :type "Key Structure"))
  (bind _arrow1 (`self.Arrow1`))
  (bind (_returnvalue_roll _returnvalue_pitch) (`KismetMathLibrary.BreakRotator` (`SceneComponent.K2_GetComponentRotation` _arrow1)))
  (:`Pressed`
    (`SceneComponent.K2_SetRelativeRotation` _arrow1 (`KismetMathLibrary.MakeRotator` _returnvalue_roll (- _returnvalue_pitch 2.0) 0.0) false false)
    (set `self.Float` (- (`self.Float`) 50.0))))

(event `Key|SpaceBar`
  (params (Key :type "Key Structure"))
  (:`Pressed`
    (bind _returnvalue (`|SpawnActorFromClass` "/Game/Blueprints/BP_Projectile.BP_Projectile_C" (`KismetMathLibrary.MakeTransform` (.location (`SceneComponent.K2_GetComponentToWorld` (`self.ProjectileSpawnPoint`))) (.rotation (`SceneComponent.K2_GetComponentToWorld` (`self.ProjectileSpawnPoint`))) (0.15 0.15 0.15)) "Undefined" "OverrideRootScale" null null))
    (`SkeletalMeshComponent.AddImpulseToAllBodiesBelow` (`/Game/Blueprints/BP_Projectile.Fish` _returnvalue) (`KismetMathLibrary.MakeVector` -2500.0 0.0 (`self.Float`)) "None" false true)))

(fn `UserConstructionScript`)